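; BP_SpellSigil is a short-lived spell sigil actor that shows a visual for its spell type, either poison or fire pillar.
; On BeginPlay it briefly waits for the spawner to assign TYPE, sets a five-second lifespan, then reveals the matching component.
; An unset type prints a failed-cast warning.
; Overlap handling is empty, with only disconnected debug print and material-swap nodes remaining.
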(event EventBeginPlay
  ;[0.15 0.15 0.15 0.5] Delay to get the type assigned from creation
  (Utilities|FlowControl|Delay 0.05)
  (Actor|SetLifeSpan 5.0)
  (switch string (Variables|Default|GetTYPE)
    (:Default
      (Development|PrintString "Spell Sigil Type not set - Failed Spellcast?"))
    (:POISON
      (Rendering|SetVisibility (Variables|Default|GetCrossSigilSpinAlembic) true false))
    (:FIREPILLAR
      (Rendering|SetVisibility (Variables|Default|GetAnimated_Bounce) true false))))

(event Collision|EventActorBeginOverlap
  (params (OtherActor :type Actor%20Object%20Reference)))

(event EventTick
  (params (DeltaSeconds :type Float%20%28single-precision%29)))

(fn ConstructionScript)