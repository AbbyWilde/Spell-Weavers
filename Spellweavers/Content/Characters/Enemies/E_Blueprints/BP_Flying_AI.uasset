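; Flying enemy AI, called a void crystal in its debug prints, that chases the player once perceived.
; AI Perception updates set any actor tagged PLAYER as Target and latch a lock-on that is never cleared.
; Tick, throttled by a short Delay, sphere-traces ahead for pawns and adds movement input toward Target when nothing is hit.
; Reaching the player only prints a message; no attack exists yet.
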(event OnPerceptionUpdated(AIPerception)
  (params (UpdatedActors :type Array%20of%20Actor%20Object%20References))
  (Development|PrintString "perception checked")
  (for _array_element UpdatedActors
    (|DEBUGSTUFF _array_element _array_element)
    (if (Actor|ActorHasTag _array_element "PLAYER")
      (Development|PrintString "PLAYER DETECTED")
      (Variables|Default|SetTarget _array_element)
      (Variables|Default|SetPlayer%20Locked%20onto true))))

(event Custom|Detent%20Player)

(event Custom|fly%20to%20player
  (bind _returnvalue (Transformation|GetActorLocation))
  (bind _returnvalue_2 (Transformation|GetActorLocation))
  (bind _target (Variables|Default|GetTarget))
  (bind _returnvalue_3 (Transformation|GetActorLocation _target))
  (bind _returnvalue_4 (Math|Rotator|FindLookatRotation _returnvalue _returnvalue_3))
  (Development|PrintString "void crystal fly to player")
  (bind (_outhit _returnvalue_5) (Collision|SphereTraceForObjects _returnvalue_2 (+ _returnvalue_2 (* (Transformation|GetActorForwardVector) 1e+02)) 1e+02 (Utilities|Array|MakeArray "ObjectTypeQuery3") false 0 "ForOneFrame"))
  (if _returnvalue_5
    (if (Actor|ActorHasTag (.HitActor (Collision|BreakHitResult _outhit)) "Player")
      (Development|PrintString "Void crystal close to player"))
    (else
      (Pawn|Input|AddMovementInput (Math|Vector|GetForwardVector (Math|Rotator|MakeRotator 0.0 (.pitch _returnvalue_4) (.yaw _returnvalue_4))) 1.0 true))))

(event EventBeginPlay)

(event Collision|EventActorBeginOverlap
  (params (OtherActor :type Actor%20Object%20Reference)))

(event EventTick
  (params (DeltaSeconds :type Float%20%28single-precision%29))
  (Utilities|FlowControl|Delay 0.2)
  (if (Variables|Default|GetPlayer%20Locked%20onto)
    (CallFunction|FlytoPlayer)))

(fn ConstructionScript)