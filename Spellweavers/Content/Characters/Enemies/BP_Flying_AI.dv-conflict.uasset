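; Flying enemy AI that detects Player-tagged actors through AI perception and flies toward them.
; Chained looping timers poll perception, validate the target and drive movement input along the look-at rotation.
; A short forward sphere trace detects the player in attack range, clears the flight timer and restarts the move timer after a delay.
; The attack itself is only a debug print, alongside other detection logging.
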(event Custom|Detent%20Player
  (Development|PrintString "dt_running")
  (for _array_element (Class|AIPerceptionComponent|GetKnownPerceivedActors (Variables|Default|GetAIPerception) "/Script/AIModule.AISense")
    (|CollapseGraph _array_element _array_element)
    (if (Actor|ActorHasTag _array_element "Player")
      (Development|PrintString "PLAYER DETECTED")
      (Variables|Default|SetTarget _array_element)
      (Utilities|Time|SetTimerbyEvent (delegate Custom|moveto) 0.1 true))))

(event Custom|moveto
  (Variables|Default|GetTarget
    (:then
      (bind _returnvalue (Utilities|Time|SetTimerbyEvent (delegate Custom|fly%20to%20player) 0.1 true)))
    (:else)))

(event Custom|fly%20to%20player
  (bind _returnvalue (Transformation|GetActorLocation))
  (bind _returnvalue_2 (Transformation|GetActorLocation))
  (bind _target (Variables|Default|GetTarget))
  (bind _returnvalue_3 (Transformation|GetActorLocation _target))
  (bind _returnvalue_4 (Math|Rotator|FindLookatRotation _returnvalue _returnvalue_3))
  (bind (_outhit _returnvalue_5) (Collision|SphereTraceForObjects _returnvalue_2 (+ _returnvalue_2 (* (Transformation|GetActorForwardVector) 1e+02)) 1e+02 (Utilities|Array|MakeArray "ObjectTypeQuery3") false 0 "None"))
  (if _returnvalue_5
    (if (Actor|ActorHasTag (.HitActor (Collision|BreakHitResult _outhit)) "Player")
      (Development|PrintString "PLAYER DETECTED ATTACK")
      (Utilities|Time|ClearandInvalidateTimerbyHandle (stale Custom|moveto _returnvalue))
      (Utilities|FlowControl|RetriggerableDelay 1.0)
      (Utilities|Time|SetTimerbyEvent (delegate Custom|moveto) 0.1 true)
      (else
        (Pawn|Input|AddMovementInput (Math|Vector|GetForwardVector (Math|Rotator|MakeRotator 0.0 (.pitch _returnvalue_4) (.yaw _returnvalue_4))) 1.0 false :!label _label)))
    (else
      (goto _label))))

(event EventBeginPlay
  (Utilities|Time|SetTimerbyEvent (delegate Custom|Detent%20Player) 0.1 true))

(event Collision|EventActorBeginOverlap
  (params (OtherActor :type Actor%20Object%20Reference)))

(fn ConstructionScript)